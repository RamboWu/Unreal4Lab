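; Behavior Tree decorator for follower AI that checks how far the controlled pawn is from the actor it follows.
; It casts the owner to Follower_AI_CON, reads TargetToFollow from the Blackboard and measures the straight-line distance between the two.
; Despite the CloseEnough name, the condition passes at or beyond AcceptableDistance and fails when closer.
; A failed cast ends the check without reporting a result.
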(event EventReceiveConditionCheck
  (params (OwnerActor :type Actor%20Object%20Reference))
  (bind _asfollower_ai_con_c (Utilities|Casting|CastToFollower_AI_CON OwnerActor))
  (Variables|Default|SetAI_CON_Ref _asfollower_ai_con_c)
  (if (>= (Math|Vector|VectorLength (- (Transformation|GetActorLocation (AI|BehaviorTree|GetBlackboardValueasActor (Variables|Default|GetTargetToFollow))) (Transformation|GetActorLocation (Pawn|GetControlledPawn (Variables|Default|GetAI_CON_Ref))))) (Variables|Default|GetAcceptableDistance))
    (Class|BTDecoratorBlueprintBase|FinishConditionCheck true)
    (else
      (Class|BTDecoratorBlueprintBase|FinishConditionCheck false))))